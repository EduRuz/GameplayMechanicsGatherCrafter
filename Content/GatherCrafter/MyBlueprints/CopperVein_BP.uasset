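; CopperVein_BP is a copper vein actor that shows an untapped vein mesh and a floating name label.
; The construction script sets the VeinType text from VeinName.
; Every Tick, mesh visibility follows IsActive, and the label appears only when the player character is within a fixed distance, rotating to face that character.
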(event `self.ReceiveTick`
  (params (DeltaSeconds :type "Float (single-precision)"))
  (bind _veintype (`self.VeinType`))
  (`SceneComponent.SetVisibility` (`self.UnTappedVeinMesh`) (`self.isActive`) false)
  (if (< (`KismetMathLibrary.VSize` (- (`self.K2_GetActorLocation` (`GameplayStatics.GetPlayerCharacter` 0)) (`self.K2_GetActorLocation`))) 500.0)
    (`SceneComponent.SetVisibility` _veintype true false)
    (`SceneComponent.K2_SetWorldRotation` _veintype (`KismetMathLibrary.FindLookAtRotation` (`self.K2_GetActorLocation`) (`self.K2_GetActorLocation` (`GameplayStatics.GetPlayerCharacter` 0))) false false)
    (else
      (`SceneComponent.SetVisibility` _veintype false false))))

(fn `UserConstructionScript`
  (`TextRenderComponent.K2_SetText` (`self.VeinType`) (`self.VeinName`)))